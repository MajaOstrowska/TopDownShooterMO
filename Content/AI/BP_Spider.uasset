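; Spider enemy that chases the player character, plays an attack montage within range and is destroyed when its health runs out.
; A looping AI MoveTo restarts shortly after each success or failure.
; Tick checks distance and montage state, pausing CharacterMovement until the attack completes.
; AnyDamage lowers clamped health, while a DamagePlayer function, not called within this Blueprint, applies per-hit damage to the player.
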(event `self.ReceiveBeginPlay`
  ;[1 1 1] Make AI run to player at start of game and repeat
  (`|AIMoveTo` self (0.0 0.0 0.0) (`GameplayStatics.GetPlayerCharacter` 0) :!label _label
    (:`OnSuccess`
      _)
    (:`OnFail`
      _))
  (`KismetSystemLibrary.Delay` 0.2)
  (goto _label))

(event `self.ReceiveTick`
  (params (DeltaSeconds :type "Float (single-precision)"))
  ;[1 1 1] Play and stop spider attack montage on approach to soldier
  (if (and (`self.IsAttackRange`) (not (`self.IsAttacking`)))
    (`ActorComponent.Deactivate` (`self.CharacterMovement`))
    (`|PlayMontage` (`self.Mesh`) "/Game/Characters/Enemy_Great_Spider/Animations/SpiderAttack_01.SpiderAttack_01"
      (:`OnCompleted`
        (`ActorComponent.Activate` (`self.CharacterMovement`) false)))))

(event `self.ReceiveAnyDamage`
  (params (Damage :type "Float (single-precision)") (DamageType :type "DamageType Object Reference") (InstigatedBy :type "Controller Object Reference") (DamageCauser :type "Actor Object Reference"))
  (bind _spiderhp (`self.DecreaseHP` Damage))
  (if (== _spiderhp 0.0)
    (`self.K2_DestroyActor`)))

(fn `DamagePlayer`
  (`GameplayStatics.ApplyDamage` (`GameplayStatics.GetPlayerCharacter` 0) (`self.DamagePerHit`)))

(fn `DecreaseHP`
  (params (Damage :type "Float (double-precision)"))
  (returns (SpiderHP :type "Float (double-precision)"))
  (bind _output_get (set `self.SpiderHP` (`KismetMathLibrary.FClamp` (- (`self.SpiderHP`) Damage) 0.0 100.0)))
  (return _output_get))

(fn `IsAttacking`
  (returns (Return :type Boolean))
  (return (`AnimInstance.Montage_IsPlaying` (`SkeletalMeshComponent.GetAnimInstance` (`self.Mesh`)) "/Game/Characters/Enemy_Great_Spider/Animations/SpiderAttack_01.SpiderAttack_01")))

(fn `IsAttackRange`
  (returns (IsAttackRange :type Boolean))
  (return (>= (`self.AttackRange`) (`self.GetDistanceTo` (`GameplayStatics.GetPlayerCharacter` 0)))))

(fn `UserConstructionScript`)